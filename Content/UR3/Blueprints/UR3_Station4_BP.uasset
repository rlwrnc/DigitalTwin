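; UR3 Station 4 robot arm that picks up parts entering its detection box and drops them at a drop point.
; Overlapping pickup bodies queue in an array; the arm takes the first one that is simulating physics.
; Timelines yaw the arm between pickup, drop and origin, while delays pace AnimBP flags and the frame's pickup and drop calls.
; After returning, it checks the queue again; VRGameMode receives its debug-print toggle.
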(event OnComponentBeginOverlap(DetectBox)
  (params (OverlappedComponent :type Primitive%20Component%20Object%20Reference) (OtherActor :type Actor%20Object%20Reference) (OtherComp :type Primitive%20Component%20Object%20Reference) (OtherBodyIndex :type Integer) (bFromSweep :type Boolean) (SweepResult :type Hit%20Result%20Structure%20%28by%20ref%29))
  ;[1 1 1] Detect
  (|Checkifready OtherActor
    (:else
      (CallFunction|DetectObject (Utilities|Array|Get(acopy) (Variables|Default|GetOverlappedActors))))))

(event OnComponentEndOverlap(DetectBox)
  (params (OverlappedComponent :type Primitive%20Component%20Object%20Reference) (OtherActor :type Actor%20Object%20Reference) (OtherComp :type Primitive%20Component%20Object%20Reference) (OtherBodyIndex :type Integer))
  ;[1 1 1] Detect
  ;;[1 1 1] When Object leaves collider, reset animations
  (Variables|Default|SetPartDetected false)
  (Variables|/Game/UR3/Anim/UR3_AnimBP.UR3_AnimBP_C|SetIsObjectInFront? (stale EventBeginPlay _asur3_anim_bp) false))

(event Custom|Debug_Switch
  ;[1 1 1] Debug
  (Variables|Default|SetDEBUG? (not (Variables|Default|GetDEBUG?))))

(event Custom|Pickup%20Object
  (params (Pickup :type BP%20Pickup%20Frame%20Object%20Reference) (AnimIn :type UR3%20Anim%20BP%20Object%20Reference))
  ;[1 1 1] Pickup
  (|Movetopickuppointandpickupcube Pickup AnimIn)
  (CallFunction|MoveObject))

(event Custom|Move%20Object
  ;[1 1 1] MoveTo
  (|MoveArmtoDropPoint)
  (CallFunction|DropObject))

(event Custom|Drop%20Object
  ;[1 1 1] Drop
  (|DropCube)
  ;[1 1 1] Return
  (|ReturnArmtoOrigin
    (:Finished
      ;[1 1 1] Check For More
      (Variables|Default|SetMoving false)
      (CallFunction|CheckforObjects))))

(event Custom|Detect%20Object
  (params (OverlappedActor :type Actor%20Object%20Reference))
  ;[1 1 1] Detect
  (bind _asbp_pickup_frame (|CheckIfAble OverlappedActor))
  (CallFunction|PickupObject _asbp_pickup_frame (stale EventBeginPlay _asur3_anim_bp)))

(event Custom|Check%20For%20Objects
  ;[1 1 1] If Multiple Items, Restart
  (|CheckForMoreobjects))

(event EventBeginPlay
  (Utilities|FlowControl|Sequence
    (:then_0
      ;[1 1 1] Animation Update
      (bind _asur3_anim_bp (Utilities|Casting|CastToUR3_AnimBP (Components|SkeletalMesh|GetAnimInstance (Variables|Default|GetUR3)))))
    (:then_1
      ;[1 1 1] Debug
      (bind _asvrgame_mode (Utilities|Casting|CastToVRGameMode (Game|GetGameMode)))
      (EventDispatchers|AssignDebug _asvrgame_mode (delegate Custom|Debug_Switch)))))

(fn ConstructionScript)